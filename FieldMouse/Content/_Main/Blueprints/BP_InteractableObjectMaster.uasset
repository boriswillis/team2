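; BP_InteractableObjectMaster is an interactable object base that shows an interaction prompt when the player character is nearby.
; On BeginPlay it fills the W_InteractionPrompt text from the InteractText field of its ObjectInfo.
; Box overlap begin and end events show and hide the prompt's widget component, responding only to BP_ThirdPersonCharacter.
; The graph handles only the prompt and contains no interaction logic.
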(event OnComponentBeginOverlap(Box)
  (params (OverlappedComponent :type Primitive%20Component%20Object%20Reference) (OtherActor :type Actor%20Object%20Reference) (OtherComp :type Primitive%20Component%20Object%20Reference) (OtherBodyIndex :type Integer) (bFromSweep :type Boolean) (SweepResult :type Hit%20Result%20Structure%20%28by%20ref%29))
  (Utilities|Casting|CastToBP_ThirdPersonCharacter OtherActor)
  (Rendering|SetVisibility (Variables|Default|GetWidget) true false))

(event OnComponentEndOverlap(Box)
  (params (OverlappedComponent :type Primitive%20Component%20Object%20Reference) (OtherActor :type Actor%20Object%20Reference) (OtherComp :type Primitive%20Component%20Object%20Reference) (OtherBodyIndex :type Integer))
  (Utilities|Casting|CastToBP_ThirdPersonCharacter OtherActor)
  (Rendering|SetVisibility (Variables|Default|GetWidget) false false))

(event EventBeginPlay
  (bind _asw_interaction_prompt (Utilities|Casting|CastToW_InteractionPrompt (UserInterface|GetWidget (Variables|Default|GetWidget))))
  (Rendering|Components|TextRender|SetText (Variables|/Game/_Main/Widget/W_InteractionPrompt.W_InteractionPrompt_C|GetInteractText _asw_interaction_prompt) (.InteractText (Utilities|Struct|BreakS_InteractableObjectStructure (Variables|Default|GetObjectInfo)))))

(event Collision|EventActorBeginOverlap
  (params (OtherActor :type Actor%20Object%20Reference)))

(event EventTick
  (params (DeltaSeconds :type Float%20%28single-precision%29)))

(fn ConstructionScript)