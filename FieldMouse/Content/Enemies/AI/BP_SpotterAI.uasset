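; Stealth guard enemy that patrols waypoints, spots the player and triggers a game over.
; PawnSensing sight fills a detection bar on its widget through a timeline, which reverses when a retriggerable delay expires without new sightings.
; A full bar sets IsDetected; being seen then, or touching the guard's capsule, shows the lose screen and pauses.
; AIPerception stimuli from the player send it to investigate the location before calling patrol again.
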(event OnSeePawn(PawnSensing)
  (params (Pawn :type Pawn%20Object%20Reference))
  ;[0.15 0.15 0.15 0.5] Chase Player
  (Utilities|FlowControl|Sequence
    (:then_0
      (Utilities|FlowControl|Sequence
        (:then_0
          (Utilities|FlowControl|DoOnce false :!label _label
            (:Completed
              (Class|BIDetectionInterface|StartDetection(Message) Pawn self)
              (CallFunction|StartDetecting)
              (bind _asw_enemy_detection_icon (Utilities|Casting|CastToW_EnemyDetectionIcon (UserInterface|GetWidget (Variables|Default|GetWidget))))
              (Widget|SetVisibility (Variables|/Game/_Main/Widget/W_EnemyDetectionIcon.W_EnemyDetectionIcon_C|GetDetectionProgressBar _asw_enemy_detection_icon) "Visible"))))
        (:then_1
          (if (Variables|Default|GetIsDetected?)
            (Utilities|Casting|CastToBP_ThirdPersonCharacter Pawn)
            (Viewport|RemoveAllWidgets)
            (bind _returnvalue (UserInterface|CreateWidget "/Game/_Main/Widget/W_LoseScreen.W_LoseScreen_C"))
            (UserInterface|Viewport|AddtoViewport _returnvalue 0)
            (Game|SetGamePaused true)))))
    (:then_1
      (Utilities|FlowControl|RetriggerableDelay 0.5)
      (Class|BIDetectionInterface|StopDetection(Message) Pawn)
      (CallFunction|StopDetecting)
      (goto _label Reset))))

(event OnComponentHit(CapsuleComponent)
  (params (HitComponent :type Primitive%20Component%20Object%20Reference) (OtherActor :type Actor%20Object%20Reference) (OtherComp :type Primitive%20Component%20Object%20Reference) (NormalImpulse :type Vector :default "0, 0, 0") (Hit :type Hit%20Result%20Structure%20%28by%20ref%29))
  (Utilities|Casting|CastToBP_ThirdPersonCharacter OtherActor)
  (Viewport|RemoveAllWidgets)
  (bind _returnvalue (UserInterface|CreateWidget "/Game/_Main/Widget/W_LoseScreen.W_LoseScreen_C"))
  (UserInterface|Viewport|AddtoViewport _returnvalue 0)
  (Game|SetGamePaused true))

(event OnTargetPerceptionUpdated(AIPerception)
  (params (Actor :type Actor%20Object%20Reference) (Stimulus :type AI%20Stimulus%20Structure))
  (bind (_age _expirationage _strength _stimuluslocation _receiverlocation _tag _bsuccessfullysensed) (Utilities|Struct|BreakAIStimulus Stimulus))
  (Development|PrintString "Hello")
  (Utilities|Casting|CastToBP_ThirdPersonCharacter Actor)
  (if _bsuccessfullysensed
    (Variables|Default|SetInvestigating? true)
    (AI|AIMoveTo self _stimuluslocation 0 5.0 false
      (:OnSuccess
        (Utilities|FlowControl|Delay 1.0)
        (CallFunction|GuardPatrol)))))

(event Custom|StartDetecting
  (params (AI :type Character%20Object%20Reference))
  (bind _asw_enemy_detection_icon (Utilities|Casting|CastToW_EnemyDetectionIcon (UserInterface|GetWidget (Variables|Default|GetWidget))))
  (if (Widget|IsVisible (Variables|/Game/_Main/Widget/W_EnemyDetectionIcon.W_EnemyDetectionIcon_C|GetDetectionProgressBar _asw_enemy_detection_icon))
    (bind (_direction _detectiontrack) (Timeline|Timeline Play)
      (:Update
        (Progress|SetPercent (Variables|/Game/_Main/Widget/W_EnemyDetectionIcon.W_EnemyDetectionIcon_C|GetDetectionProgressBar _asw_enemy_detection_icon) _detectiontrack))
      (:Finished
        (switch Utilities|FlowControl|Switch|SwitchonETimelineDirection _direction
          (:Forward
            (Class|ProgressBar|SetFillColorandOpacity (Variables|/Game/_Main/Widget/W_EnemyDetectionIcon.W_EnemyDetectionIcon_C|GetDetectionProgressBar _asw_enemy_detection_icon) "(R=1.000000,G=0.000000,B=0.000000,A=1.000000)")
            (CallFunction|StartChasing))
          (:Backward
            (Utilities|FlowControl|RetriggerableDelay 0.5)
            (Widget|SetVisibility (Variables|/Game/_Main/Widget/W_EnemyDetectionIcon.W_EnemyDetectionIcon_C|GetDetectionProgressBar _asw_enemy_detection_icon) "Hidden")
            (Class|ProgressBar|SetFillColorandOpacity (Variables|/Game/_Main/Widget/W_EnemyDetectionIcon.W_EnemyDetectionIcon_C|GetDetectionProgressBar _asw_enemy_detection_icon) "(R=1.000000,G=1.000000,B=1.000000,A=1.000000)")))))
    (else
      (Widget|SetVisibility (Variables|/Game/_Main/Widget/W_EnemyDetectionIcon.W_EnemyDetectionIcon_C|GetDetectionProgressBar _asw_enemy_detection_icon) "Visible")
      (Timeline|Timeline Play))))

(event Custom|GuardPatrol
  ;[0.15 0.15 0.15 0.5] Patrol
  (Variables|/Script/Engine.CharacterMovementComponent|SetMaxWalkSpeed (Variables|Character|GetCharacterMovement) 2e+02)
  (AI|AIMoveTo self "0, 0, 0" (Utilities|Array|Get(acopy) (Variables|Default|GetWaypoints) (Variables|Default|GetCurrentWaypoint)) 1e+01 false
    (:OnSuccess
      (Math|Integer|IncrementInt (Variables|Default|GetCurrentWaypoint)
        (:%20%20
          (if (>= (Variables|Default|GetCurrentWaypoint) (Utilities|Array|Length (Variables|Default|GetWaypoints)))
            (Variables|Default|SetCurrentWaypoint 0))
          (Utilities|FlowControl|Delay 5.0)
          (if (not (Variables|Default|GetInvestigating?))
            (CallFunction|GuardPatrol)))))))

(event Custom|StopDetecting
  (Audio|Components|Audio|Stop (Variables|Default|GetTimeline))
  (bind (_direction _detectiontrack) (Timeline|Timeline Reverse)
    (:Update
      (Progress|SetPercent (Variables|/Game/_Main/Widget/W_EnemyDetectionIcon.W_EnemyDetectionIcon_C|GetDetectionProgressBar (stale Custom|StartDetecting _asw_enemy_detection_icon)) _detectiontrack))
    (:Finished
      (switch Utilities|FlowControl|Switch|SwitchonETimelineDirection _direction
        (:Forward
          (Class|ProgressBar|SetFillColorandOpacity (Variables|/Game/_Main/Widget/W_EnemyDetectionIcon.W_EnemyDetectionIcon_C|GetDetectionProgressBar (stale Custom|StartDetecting _asw_enemy_detection_icon)) "(R=1.000000,G=0.000000,B=0.000000,A=1.000000)")
          (CallFunction|StartChasing))
        (:Backward
          (Utilities|FlowControl|RetriggerableDelay 0.5)
          (Widget|SetVisibility (Variables|/Game/_Main/Widget/W_EnemyDetectionIcon.W_EnemyDetectionIcon_C|GetDetectionProgressBar (stale Custom|StartDetecting _asw_enemy_detection_icon)) "Hidden")
          (Class|ProgressBar|SetFillColorandOpacity (Variables|/Game/_Main/Widget/W_EnemyDetectionIcon.W_EnemyDetectionIcon_C|GetDetectionProgressBar (stale Custom|StartDetecting _asw_enemy_detection_icon)) "(R=1.000000,G=1.000000,B=1.000000,A=1.000000)"))))))

(event Custom|StartChasing
  (Variables|Default|SetIsDetected? true)
  (bind _asw_enemy_detection_icon (Utilities|Casting|CastToW_EnemyDetectionIcon (UserInterface|GetWidget (Variables|Default|GetWidget))))
  (Class|ProgressBar|SetFillColorandOpacity (Variables|/Game/_Main/Widget/W_EnemyDetectionIcon.W_EnemyDetectionIcon_C|GetDetectionProgressBar _asw_enemy_detection_icon) "(R=1.000000,G=0.017305,B=0.027253,A=1.000000)"))

(event Custom|StopChasing
  (Variables|Default|SetIsDetected? false)
  (bind _asw_enemy_detection_icon (Utilities|Casting|CastToW_EnemyDetectionIcon (UserInterface|GetWidget (Variables|Default|GetWidget))))
  (Class|ProgressBar|SetFillColorandOpacity (Variables|/Game/_Main/Widget/W_EnemyDetectionIcon.W_EnemyDetectionIcon_C|GetDetectionProgressBar _asw_enemy_detection_icon) "(R=1.000000,G=1.000000,B=1.000000,A=1.000000)")
  (Widget|SetVisibility (Variables|/Game/_Main/Widget/W_EnemyDetectionIcon.W_EnemyDetectionIcon_C|GetDetectionProgressBar _asw_enemy_detection_icon) "Hidden")
  (CallFunction|GuardPatrol))

(event EventStopChase)

(event EventBeginPlay
  (if (not (Variables|Default|GetCanSeePlayer?))
    (CallFunction|GuardPatrol)
    (bind _asw_enemy_detection_icon (Utilities|Casting|CastToW_EnemyDetectionIcon (UserInterface|GetWidget (Variables|Default|GetWidget))))
    (Widget|SetVisibility (Variables|/Game/_Main/Widget/W_EnemyDetectionIcon.W_EnemyDetectionIcon_C|GetDetectionProgressBar _asw_enemy_detection_icon) "Hidden")))

(event EventStartChase)

(fn ConstructionScript)