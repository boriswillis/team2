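; Enemy guard that detects, investigates and chases the player, showing the lose screen and pausing the game on capsule contact.
; PawnSensing sight plays a Timeline that fills a detection widget and triggers chasing when full.
; A retriggerable delay reverses detection once sight lapses.
; AIPerception stimuli send it to investigate, while waypoint patrol logic sits disconnected, leaving GuardPatrol empty.
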(event OnSeePawn(PawnSensing)
  (params (Pawn :type Pawn%20Object%20Reference))
  ;[0.15 0.15 0.15 0.5] Chase Player
  (Utilities|FlowControl|Sequence
    (:then_0
      (Utilities|FlowControl|Sequence
        (:then_0
          (Utilities|FlowControl|DoOnce false :!label _label
            (:Completed
              (CallFunction|StartDetecting)
              (bind _asw_enemy_detection_icon (Utilities|Casting|CastToW_EnemyDetectionIcon (UserInterface|GetWidget (Variables|Default|GetWidget))))
              (Widget|SetVisibility (Variables|/Game/_Main/Widget/W_EnemyDetectionIcon.W_EnemyDetectionIcon_C|GetDetectionProgressBar _asw_enemy_detection_icon) "Visible"))))
        (:then_1
          (if (Variables|Default|GetIsDetected?)
            (AI|AIMoveTo self "0, 0, 0" Pawn 5.0 false
              (:then
                (Development|PrintString "Chasing")))))))
    (:then_1
      (Utilities|FlowControl|RetriggerableDelay 1.0)
      (CallFunction|StopDetecting)
      (goto _label Reset))))

(event OnComponentHit(CapsuleComponent)
  (params (HitComponent :type Primitive%20Component%20Object%20Reference) (OtherActor :type Actor%20Object%20Reference) (OtherComp :type Primitive%20Component%20Object%20Reference) (NormalImpulse :type Vector :default "0, 0, 0") (Hit :type Hit%20Result%20Structure%20%28by%20ref%29))
  ;[0.15 0.15 0.15 0.5] End Game on Collision with Player
  (Utilities|Casting|CastToBP_ThirdPersonCharacter OtherActor)
  (Viewport|RemoveAllWidgets)
  (bind _returnvalue (UserInterface|CreateWidget "/Game/_Main/Widget/W_LoseScreen.W_LoseScreen_C"))
  (UserInterface|Viewport|AddtoViewport _returnvalue 0)
  (Game|SetGamePaused true))

(event OnTargetPerceptionUpdated(AIPerception)
  (params (Actor :type Actor%20Object%20Reference) (Stimulus :type AI%20Stimulus%20Structure))
  (bind (_age _expirationage _strength _stimuluslocation _receiverlocation _tag _bsuccessfullysensed) (Utilities|Struct|BreakAIStimulus Stimulus))
  ;[0.15 0.15 0.15 0.5] Investigate After Hearing
  (Utilities|Casting|CastToBP_ThirdPersonCharacter Actor)
  (if _bsuccessfullysensed
    (Variables|Default|SetInvestigating? true)
    (AI|AIMoveTo self _stimuluslocation 0 5.0 false
      (:OnSuccess
        (Utilities|FlowControl|Delay 1e+01)
        (Variables|Default|SetInvestigating? false)))))

(event Custom|StartDetecting
  (params (AI :type Character%20Object%20Reference))
  ;[0.15 0.15 0.15 0.5] Start/Stop Detecting
  (bind _asw_enemy_detection_icon (Utilities|Casting|CastToW_EnemyDetectionIcon (UserInterface|GetWidget (Variables|Default|GetWidget))))
  (if (Widget|IsVisible (Variables|/Game/_Main/Widget/W_EnemyDetectionIcon.W_EnemyDetectionIcon_C|GetDetectionProgressBar _asw_enemy_detection_icon))
    (bind (_direction _detectiontrack) (Timeline|Timeline Play)
      (:Update
        (Progress|SetPercent (Variables|/Game/_Main/Widget/W_EnemyDetectionIcon.W_EnemyDetectionIcon_C|GetDetectionProgressBar _asw_enemy_detection_icon) _detectiontrack))
      (:Finished
        (switch Utilities|FlowControl|Switch|SwitchonETimelineDirection _direction
          (:Forward
            (Class|ProgressBar|SetFillColorandOpacity (Variables|/Game/_Main/Widget/W_EnemyDetectionIcon.W_EnemyDetectionIcon_C|GetDetectionProgressBar _asw_enemy_detection_icon) "(R=1.000000,G=0.000000,B=0.000000,A=1.000000)")
            (CallFunction|StartChasing))
          (:Backward
            (Utilities|FlowControl|RetriggerableDelay 0.5)
            (Widget|SetVisibility (Variables|/Game/_Main/Widget/W_EnemyDetectionIcon.W_EnemyDetectionIcon_C|GetDetectionProgressBar _asw_enemy_detection_icon) "Hidden")
            (Class|ProgressBar|SetFillColorandOpacity (Variables|/Game/_Main/Widget/W_EnemyDetectionIcon.W_EnemyDetectionIcon_C|GetDetectionProgressBar _asw_enemy_detection_icon) "(R=1.000000,G=1.000000,B=1.000000,A=1.000000)")
            (Components|Movement|StopMovementImmediately (Variables|Character|GetCharacterMovement))))))
    (else
      (Widget|SetVisibility (Variables|/Game/_Main/Widget/W_EnemyDetectionIcon.W_EnemyDetectionIcon_C|GetDetectionProgressBar _asw_enemy_detection_icon) "Visible")
      (Timeline|Timeline Play))))

(event Custom|GuardPatrol
  ;[0.15 0.15 0.15 0.5] Patrol
)

(event Custom|StopDetecting
  ;[0.15 0.15 0.15 0.5] Start/Stop Detecting
  (Variables|Default|SetCanSeePlayer? false)
  (Variables|Default|SetIsDetected? false)
  (Variables|Default|SetInvestigating? false)
  (Audio|Components|Audio|Stop (Variables|Default|GetTimeline))
  (bind (_direction _detectiontrack) (Timeline|Timeline Reverse)
    (:Update
      (Progress|SetPercent (Variables|/Game/_Main/Widget/W_EnemyDetectionIcon.W_EnemyDetectionIcon_C|GetDetectionProgressBar (stale Custom|StartDetecting _asw_enemy_detection_icon)) _detectiontrack))
    (:Finished
      (switch Utilities|FlowControl|Switch|SwitchonETimelineDirection _direction
        (:Forward
          (Class|ProgressBar|SetFillColorandOpacity (Variables|/Game/_Main/Widget/W_EnemyDetectionIcon.W_EnemyDetectionIcon_C|GetDetectionProgressBar (stale Custom|StartDetecting _asw_enemy_detection_icon)) "(R=1.000000,G=0.000000,B=0.000000,A=1.000000)")
          (CallFunction|StartChasing))
        (:Backward
          (Utilities|FlowControl|RetriggerableDelay 0.5)
          (Widget|SetVisibility (Variables|/Game/_Main/Widget/W_EnemyDetectionIcon.W_EnemyDetectionIcon_C|GetDetectionProgressBar (stale Custom|StartDetecting _asw_enemy_detection_icon)) "Hidden")
          (Class|ProgressBar|SetFillColorandOpacity (Variables|/Game/_Main/Widget/W_EnemyDetectionIcon.W_EnemyDetectionIcon_C|GetDetectionProgressBar (stale Custom|StartDetecting _asw_enemy_detection_icon)) "(R=1.000000,G=1.000000,B=1.000000,A=1.000000)")
          (Components|Movement|StopMovementImmediately (Variables|Character|GetCharacterMovement)))))))

(event Custom|StartChasing
  ;[0.15 0.15 0.15 0.5] Start Chasing
  (Variables|Default|SetIsDetected? true)
  (bind _asw_enemy_detection_icon (Utilities|Casting|CastToW_EnemyDetectionIcon (UserInterface|GetWidget (Variables|Default|GetWidget))))
  (Class|ProgressBar|SetFillColorandOpacity (Variables|/Game/_Main/Widget/W_EnemyDetectionIcon.W_EnemyDetectionIcon_C|GetDetectionProgressBar _asw_enemy_detection_icon) "(R=1.000000,G=0.017305,B=0.027253,A=1.000000)"))

(event Custom|StopChasing
  ;[0.15 0.15 0.15 0.5] Stop Chasing
  (Variables|Default|SetIsDetected? false)
  (bind _asw_enemy_detection_icon (Utilities|Casting|CastToW_EnemyDetectionIcon (UserInterface|GetWidget (Variables|Default|GetWidget))))
  (Class|ProgressBar|SetFillColorandOpacity (Variables|/Game/_Main/Widget/W_EnemyDetectionIcon.W_EnemyDetectionIcon_C|GetDetectionProgressBar _asw_enemy_detection_icon) "(R=1.000000,G=1.000000,B=1.000000,A=1.000000)")
  (Widget|SetVisibility (Variables|/Game/_Main/Widget/W_EnemyDetectionIcon.W_EnemyDetectionIcon_C|GetDetectionProgressBar _asw_enemy_detection_icon) "Hidden"))

(event Custom|PatrolEnter
  ;[0.15 0.15 0.15 0.5] Rotate Towards Patrol Point Arrow
  (Utilities|FlowControl|Gate true) ; enters at Open
)

(event Custom|PatrolExit
  ;[0.15 0.15 0.15 0.5] Rotate Towards Patrol Point Arrow
  (Utilities|FlowControl|Gate true) ; enters at Close
)

(event EventBeginPlay
  ;[0.15 0.15 0.15 0.5] Begin Play Initialize Settings
  (if (not (Variables|Default|GetCanSeePlayer?))
    (CallFunction|GuardPatrol)
    (bind _asw_enemy_detection_icon (Utilities|Casting|CastToW_EnemyDetectionIcon (UserInterface|GetWidget (Variables|Default|GetWidget))))
    (Widget|SetVisibility (Variables|/Game/_Main/Widget/W_EnemyDetectionIcon.W_EnemyDetectionIcon_C|GetDetectionProgressBar _asw_enemy_detection_icon) "Hidden")))

(event EventTick
  (params (DeltaSeconds :type Float%20%28single-precision%29))
  ;[0.15 0.15 0.15 0.5] Rotate Towards Patrol Point Arrow
  (Utilities|FlowControl|Gate true
    (:Exit
      (Transformation|SetActorRotation self (Math|Interpolation|RInterpTo (Transformation|GetActorRotation self) (Transformation|GetWorldRotation (Variables|/Game/Enemies/AI/BP_Waypoint.BP_Waypoint_C|GetArrow (Variables|Default|GetCurrentPatrolPoint))) DeltaSeconds 2.0)))))

(fn ConstructionScript)