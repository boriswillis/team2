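; Stealth enemy AI that patrols waypoints with random pauses and shows the lose screen, pausing the game, on full detection or player collision.
; Sighting a non-camouflaged player runs a detection timeline that fills a progress icon faster at closer range.
; A retriggerable delay on sight events acts as a lost-sight timeout, reversing detection.
; Perceived stimuli, or losing a fully detected player, send it to investigate before patrol resumes.
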(event OnSeePawn(PawnSensing)
  (params (Pawn :type Pawn%20Object%20Reference))
  (bind _returnvalue (Transformation|GetDistanceTo Pawn))
  (bind _asbp_third_person_character (Utilities|Casting|CastToBP_ThirdPersonCharacter Pawn))
  ;[0.15 0.15 0.15 0.5] Chase Player
  (if (not (Variables|/Game/ThirdPerson/Blueprints/BP_ThirdPersonCharacter.BP_ThirdPersonCharacter_C|GetIsCamo? _asbp_third_person_character))
    (Variables|Default|SetLastKnownLocation (Transformation|GetActorLocation Pawn))
    (if (>= _returnvalue 1e+03)
      (bind _output_get (Variables|Default|SetPlayRate 1.0))
      (Components|Timeline|SetPlayRate (Variables|Default|GetTimeline) _output_get)
      (Variables|Default|SetCanSeePlayer? true :!label _label)
      (Class|BIDetectionInterface|UpdatePlayRate(Message) Pawn (Variables|Default|GetPlayRate))
      (Utilities|FlowControl|Sequence
        (:then_0
          (Utilities|FlowControl|Sequence
            (:then_0
              (Utilities|FlowControl|DoOnce false :!label _label_2
                (:Completed
                  (Class|BIDetectionInterface|StartDetection(Message) Pawn self (Variables|Default|GetPlayRate))
                  (CallFunction|StartDetecting)
                  (bind _asw_enemy_detection_icon (Utilities|Casting|CastToW_EnemyDetectionIcon (UserInterface|GetWidget (Variables|Default|GetWidget))))
                  (Widget|SetVisibility (Variables|/Game/_Main/Widget/W_EnemyDetectionIcon.W_EnemyDetectionIcon_C|GetDetectionProgressBar _asw_enemy_detection_icon) "Visible"))))
            (:then_1
              (if (Variables|Default|GetIsDetected?)
                (Variables|/Script/Engine.CharacterMovementComponent|SetMaxWalkSpeed (Variables|Character|GetCharacterMovement) (Variables|Default|GetChaseSpeed))
                (AI|AIMoveTo self (Variables|Default|GetLastKnownLocation) 0 5e+01 false)))))
        (:then_1
          (Utilities|FlowControl|RetriggerableDelay 0.05)
          (Variables|Default|SetCanSeePlayer? false)
          (CallFunction|StopDetecting)
          (Class|BIDetectionInterface|StopDetection(Message) Pawn)
          (goto _label_2 Reset)))
      (elif (>= _returnvalue 5e+02)
        (bind _output_get_2 (Variables|Default|SetPlayRate 1.5))
        (Components|Timeline|SetPlayRate (Variables|Default|GetTimeline) _output_get_2)
        (goto _label)
        (elif (< _returnvalue 5e+02)
          (bind _output_get_3 (Variables|Default|SetPlayRate 3.0))
          (Components|Timeline|SetPlayRate (Variables|Default|GetTimeline) _output_get_3)
          (goto _label))))))

(event OnComponentHit(CapsuleComponent)
  (params (HitComponent :type Primitive%20Component%20Object%20Reference) (OtherActor :type Actor%20Object%20Reference) (OtherComp :type Primitive%20Component%20Object%20Reference) (NormalImpulse :type Vector :default "0, 0, 0") (Hit :type Hit%20Result%20Structure%20%28by%20ref%29))
  ;[0.15 0.15 0.15 0.5] End Game on Collision with Player
  (Utilities|Casting|CastToBP_ThirdPersonCharacter OtherActor)
  (Viewport|RemoveAllWidgets)
  (bind _returnvalue (UserInterface|CreateWidget "/Game/_Main/Widget/W_LoseScreen.W_LoseScreen_C"))
  (UserInterface|Viewport|AddtoViewport _returnvalue 0)
  (Game|SetGamePaused true))

(event OnTargetPerceptionUpdated(AIPerception)
  (params (Actor :type Actor%20Object%20Reference) (Stimulus :type AI%20Stimulus%20Structure))
  (bind (_age _expirationage _strength _stimuluslocation _receiverlocation _tag _bsuccessfullysensed) (Utilities|Struct|BreakAIStimulus Stimulus))
  ;[0.15 0.15 0.15 0.5] Investigate After Hearing
  (if (not (Variables|Default|GetCanSeePlayer?))
    (Utilities|Casting|CastToBP_ThirdPersonCharacter Actor)
    (if _bsuccessfullysensed
      (Variables|Default|SetInvestigating? true)
      (bind _asw_investigating_widget (Utilities|Casting|CastToW_InvestigatingWidget (UserInterface|GetWidget (Variables|Default|GetInvestigationWidget))))
      (Widget|SetVisibility (Variables|/Game/_Main/Widget/W_InvestigatingWidget.W_InvestigatingWidget_C|GetProgressBar_5 _asw_investigating_widget) "Visible")
      (AI|AIMoveTo self _stimuluslocation 0 5e+01 false
        (:OnSuccess
          (Utilities|FlowControl|Delay 1e+01)
          (Variables|Default|SetInvestigating? false)
          (bind _asw_investigating_widget_2 (Utilities|Casting|CastToW_InvestigatingWidget (UserInterface|GetWidget (Variables|Default|GetInvestigationWidget))))
          (Widget|SetVisibility (Variables|/Game/_Main/Widget/W_InvestigatingWidget.W_InvestigatingWidget_C|GetProgressBar_5 _asw_investigating_widget_2) "Hidden")
          (CallFunction|Patrol))))))

(event Custom|StartDetecting
  (params (AI :type Character%20Object%20Reference))
  ;[0.15 0.15 0.15 0.5] Start/Stop Detecting
  (bind _asw_enemy_detection_icon (Utilities|Casting|CastToW_EnemyDetectionIcon (UserInterface|GetWidget (Variables|Default|GetWidget))))
  (if (Widget|IsVisible (Variables|/Game/_Main/Widget/W_EnemyDetectionIcon.W_EnemyDetectionIcon_C|GetDetectionProgressBar _asw_enemy_detection_icon))
    (bind (_direction _detectiontrack) (Timeline|Timeline Play)
      (:Update
        (Progress|SetPercent (Variables|/Game/_Main/Widget/W_EnemyDetectionIcon.W_EnemyDetectionIcon_C|GetDetectionProgressBar _asw_enemy_detection_icon) _detectiontrack))
      (:Finished
        (switch Utilities|FlowControl|Switch|SwitchonETimelineDirection _direction
          (:Forward
            (Class|ProgressBar|SetFillColorandOpacity (Variables|/Game/_Main/Widget/W_EnemyDetectionIcon.W_EnemyDetectionIcon_C|GetDetectionProgressBar _asw_enemy_detection_icon) "(R=1.000000,G=0.000000,B=0.000000,A=1.000000)")
            (CallFunction|StartChasing)
            (Viewport|RemoveAllWidgets)
            (bind _returnvalue (UserInterface|CreateWidget "/Game/_Main/Widget/W_LoseScreen.W_LoseScreen_C"))
            (UserInterface|Viewport|AddtoViewport _returnvalue 0)
            (Game|SetGamePaused true))
          (:Backward
            (Utilities|FlowControl|RetriggerableDelay 0.01)
            (Widget|SetVisibility (Variables|/Game/_Main/Widget/W_EnemyDetectionIcon.W_EnemyDetectionIcon_C|GetDetectionProgressBar _asw_enemy_detection_icon) "Hidden")
            (Class|ProgressBar|SetFillColorandOpacity (Variables|/Game/_Main/Widget/W_EnemyDetectionIcon.W_EnemyDetectionIcon_C|GetDetectionProgressBar _asw_enemy_detection_icon) "(R=1.000000,G=1.000000,B=1.000000,A=1.000000)")
            (CallFunction|StopChasing)))))
    (else
      (Widget|SetVisibility (Variables|/Game/_Main/Widget/W_EnemyDetectionIcon.W_EnemyDetectionIcon_C|GetDetectionProgressBar _asw_enemy_detection_icon) "Visible")
      (Timeline|Timeline Play))))

(event Custom|Patrol
  (if (not (Variables|Default|GetIsDetected?))
    (if (not (Variables|Default|GetInvestigating?))
      ;[0.15 0.15 0.15 0.5] Patrol
      (if (not (<= (Utilities|Array|Length (Variables|Default|GetWaypoints)) 0))
        (Variables|/Script/Engine.CharacterMovementComponent|SetMaxWalkSpeed (Variables|Character|GetCharacterMovement) (Variables|Default|GetPatrolSpeed))
        (Variables|Default|SetCurrentPatrolPoint (Utilities|Array|Get(acopy) (Variables|Default|GetWaypoints) (Variables|Default|GetCurrentWaypoint)))
        (AI|AIMoveTo self "0, 0, 0" (Utilities|Array|Get(acopy) (Variables|Default|GetWaypoints) (Variables|Default|GetCurrentWaypoint)) 5e+01 false
          (:OnSuccess
            (CallFunction|PatrolEnter)
            (CallFunction|PatrolExit)
            (Utilities|FlowControl|Delay (Math|Conversions|ToFloat(Integer) (Math|Random|RandomIntegerinRange 10 15)))
            (Math|Integer|IncrementInt (Variables|Default|GetCurrentWaypoint)
              (:%20%20
                (if (>= (Variables|Default|GetCurrentWaypoint) (Utilities|Array|Length (Variables|Default|GetWaypoints)))
                  (Variables|Default|SetCurrentWaypoint 0))
                (CallFunction|Patrol)))))))))

(event Custom|StopDetecting
  ;[0.15 0.15 0.15 0.5] Start/Stop Detecting
  (Audio|Components|Audio|Stop (Variables|Default|GetTimeline))
  (bind (_direction _detectiontrack) (Timeline|Timeline Reverse)
    (:Update
      (Progress|SetPercent (Variables|/Game/_Main/Widget/W_EnemyDetectionIcon.W_EnemyDetectionIcon_C|GetDetectionProgressBar (stale Custom|StartDetecting _asw_enemy_detection_icon)) _detectiontrack))
    (:Finished
      (switch Utilities|FlowControl|Switch|SwitchonETimelineDirection _direction
        (:Forward
          (Class|ProgressBar|SetFillColorandOpacity (Variables|/Game/_Main/Widget/W_EnemyDetectionIcon.W_EnemyDetectionIcon_C|GetDetectionProgressBar (stale Custom|StartDetecting _asw_enemy_detection_icon)) "(R=1.000000,G=0.000000,B=0.000000,A=1.000000)")
          (CallFunction|StartChasing)
          (Viewport|RemoveAllWidgets)
          (bind _returnvalue (UserInterface|CreateWidget "/Game/_Main/Widget/W_LoseScreen.W_LoseScreen_C"))
          (UserInterface|Viewport|AddtoViewport _returnvalue 0)
          (Game|SetGamePaused true))
        (:Backward
          (Utilities|FlowControl|RetriggerableDelay 0.01)
          (Widget|SetVisibility (Variables|/Game/_Main/Widget/W_EnemyDetectionIcon.W_EnemyDetectionIcon_C|GetDetectionProgressBar (stale Custom|StartDetecting _asw_enemy_detection_icon)) "Hidden")
          (Class|ProgressBar|SetFillColorandOpacity (Variables|/Game/_Main/Widget/W_EnemyDetectionIcon.W_EnemyDetectionIcon_C|GetDetectionProgressBar (stale Custom|StartDetecting _asw_enemy_detection_icon)) "(R=1.000000,G=1.000000,B=1.000000,A=1.000000)")
          (CallFunction|StopChasing))))))

(event Custom|StartChasing
  (if (Variables|Default|GetIsDetected?)
    _
    (else
      (Audio|PlaySound2D "/Game/_Main/Audio/531750__pixelprophecy__metal-gear-solid-guard-alert-exclamation.531750__pixelprophecy__metal-gear-solid-guard-alert-exclamation" 1.0 1.0 0.0 0 0)))
  (bind _asw_investigating_widget (Utilities|Casting|CastToW_InvestigatingWidget (UserInterface|GetWidget (Variables|Default|GetInvestigationWidget))))
  (Widget|SetVisibility (Variables|/Game/_Main/Widget/W_InvestigatingWidget.W_InvestigatingWidget_C|GetProgressBar_5 _asw_investigating_widget) "Hidden")
  ;[0.15 0.15 0.15 0.5] Start Chasing
  (Variables|Default|SetSawPlayer true)
  (Variables|Default|SetIsDetected? true)
  (bind _asw_enemy_detection_icon (Utilities|Casting|CastToW_EnemyDetectionIcon (UserInterface|GetWidget (Variables|Default|GetWidget))))
  (Class|ProgressBar|SetFillColorandOpacity (Variables|/Game/_Main/Widget/W_EnemyDetectionIcon.W_EnemyDetectionIcon_C|GetDetectionProgressBar _asw_enemy_detection_icon) "(R=1.000000,G=0.017305,B=0.027253,A=1.000000)")
  (Variables|/Script/Engine.CharacterMovementComponent|SetMaxWalkSpeed (Variables|Character|GetCharacterMovement) (Variables|Default|GetChaseSpeed)))

(event Custom|StopChasing
  ;[0.15 0.15 0.15 0.5] Stop Chasing
  (Variables|Default|SetIsDetected? false)
  (if (not (Variables|Default|GetCanSeePlayer?))
    (bind _asw_enemy_detection_icon (Utilities|Casting|CastToW_EnemyDetectionIcon (UserInterface|GetWidget (Variables|Default|GetWidget))))
    (Class|ProgressBar|SetFillColorandOpacity (Variables|/Game/_Main/Widget/W_EnemyDetectionIcon.W_EnemyDetectionIcon_C|GetDetectionProgressBar _asw_enemy_detection_icon) "(R=1.000000,G=1.000000,B=1.000000,A=1.000000)")
    (Widget|SetVisibility (Variables|/Game/_Main/Widget/W_EnemyDetectionIcon.W_EnemyDetectionIcon_C|GetDetectionProgressBar _asw_enemy_detection_icon) "Hidden")
    (if (Variables|Default|GetSawPlayer)
      (bind _asw_investigating_widget (Utilities|Casting|CastToW_InvestigatingWidget (UserInterface|GetWidget (Variables|Default|GetInvestigationWidget))))
      (Widget|SetVisibility (Variables|/Game/_Main/Widget/W_InvestigatingWidget.W_InvestigatingWidget_C|GetProgressBar_5 _asw_investigating_widget) "Visible")
      (AI|AIMoveTo self (Variables|Default|GetLastKnownLocation) 0 5e+01 false
        (:OnSuccess
          (Utilities|FlowControl|Delay 1e+01)
          (bind _asw_investigating_widget_2 (Utilities|Casting|CastToW_InvestigatingWidget (UserInterface|GetWidget (Variables|Default|GetInvestigationWidget))))
          (Widget|SetVisibility (Variables|/Game/_Main/Widget/W_InvestigatingWidget.W_InvestigatingWidget_C|GetProgressBar_5 _asw_investigating_widget_2) "Hidden")
          (Variables|Default|SetInvestigating? false)
          (Variables|Default|SetSawPlayer false)
          (CallFunction|Patrol))))))

(event Custom|PatrolEnter
  ;[0.15 0.15 0.15 0.5] Rotate Towards Patrol Point Arrow
  (Utilities|FlowControl|Gate true) ; enters at Open
)

(event Custom|PatrolExit
  ;[0.15 0.15 0.15 0.5] Rotate Towards Patrol Point Arrow
  (Utilities|FlowControl|Gate true) ; enters at Close
)

(event Custom|Guard
  ;[0.15 0.15 0.15 0.5] Guard (Pause After reaching patrol point before continuing)
)

(event EventBeginPlay
  ;[0.15 0.15 0.15 0.5] Begin Play Initialize Settings
  (bind _asw_enemy_detection_icon (Utilities|Casting|CastToW_EnemyDetectionIcon (UserInterface|GetWidget (Variables|Default|GetWidget))))
  (Widget|SetVisibility (Variables|/Game/_Main/Widget/W_EnemyDetectionIcon.W_EnemyDetectionIcon_C|GetDetectionProgressBar _asw_enemy_detection_icon) "Hidden")
  (bind _asw_investigating_widget (Utilities|Casting|CastToW_InvestigatingWidget (UserInterface|GetWidget (Variables|Default|GetInvestigationWidget))))
  (Widget|SetVisibility (Variables|/Game/_Main/Widget/W_InvestigatingWidget.W_InvestigatingWidget_C|GetProgressBar_5 _asw_investigating_widget) "Hidden")
  (Variables|/Script/Engine.CharacterMovementComponent|SetMaxWalkSpeed (Variables|Character|GetCharacterMovement) (Variables|Default|GetPatrolSpeed))
  (if (not (<= (Utilities|Array|Length (Variables|Default|GetWaypoints)) 0))
    (if (not (Variables|Default|GetCanSeePlayer?))
      (CallFunction|Patrol))))

(event EventTick
  (params (DeltaSeconds :type Float%20%28single-precision%29))
  ;[0.15 0.15 0.15 0.5] Rotate Towards Patrol Point Arrow
  (Utilities|FlowControl|Gate true
    (:Exit
      (Transformation|SetActorRotation self (Math|Interpolation|RInterpTo (Transformation|GetActorRotation self) (Transformation|GetWorldRotation (Variables|/Game/Enemies/AI/BP_Waypoint.BP_Waypoint_C|GetArrow (Variables|Default|GetCurrentPatrolPoint))) DeltaSeconds 2.0)))))

(fn ConstructionScript)